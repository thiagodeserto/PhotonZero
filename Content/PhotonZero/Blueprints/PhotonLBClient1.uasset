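; Photon load-balancing client Blueprint that visualizes networked players as Card actors on a grid board and stores client state and room list.
; SetupScene sizes the board, blends to a newly spawned camera fitted to the grid and resizes card text.
; Player events spawn labeled cards, then move or recolor them by player number, with a border marking the local player.
; Tick refreshes the board's checker visibility from UseGroups every frame for simplicity.
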(event `self.setupScene`
  (params (gridSize :type Integer))
  (bind _returnvalue (+ (* gridSize 75.0) -50.0))
  ;[1 1 1] Called on start and when board size changed
  (set `self.GridSize` gridSize)
  (`/Game/Blueprints/Board.setup` (`self.board`) gridSize)
  (bind _returnvalue_2 (`|SpawnActorFromClass` "/Script/Engine.CameraActor" (`KismetMathLibrary.MakeTransform` (`KismetMathLibrary.MakeVector` -200.0 (* gridSize 50.0) _returnvalue) (`KismetMathLibrary.MakeRot` (* (`KismetMathLibrary.DegAtan2` _returnvalue (- (* gridSize 35.0) -200.0)) -1.0) 0.0))))
  (set `CameraComponent.bConstrainAspectRatio` false (`CameraActor.CameraComponent` _returnvalue_2))
  (`PlayerController.SetViewTargetWithBlend` (`GameplayStatics.GetPlayerController` 0) _returnvalue_2 0.8 "VTBlend_Linear" 0.0 false)
  (for _array_element (`self.Actors`)
    (`/Game/Blueprints/Card.UpdateTextSize` _array_element (`self.GridSize`))))

(event `self.addPlayer`
  (params (playerNr :type Integer) (playerName :type String) (local :type Boolean))
  (bind _returnvalue (`|SpawnActorFromClass` "/Game/Blueprints/Card.Card_C" (`KismetMathLibrary.MakeTransform` (0.0 0.0 0.0))))
  (set `/Game/Blueprints/Card.actorNr` playerNr _returnvalue)
  (`KismetArrayLibrary.Array_Add` (`self.Actors`) _returnvalue)
  (`/Game/Blueprints/Card.UpdateTextSize` _returnvalue (`self.GridSize`))
  (`/Game/Blueprints/Card.SetText` _returnvalue (`KismetStringLibrary.Concat_StrStr` (`KismetStringLibrary.Concat_StrStr` playerName "/") (`KismetStringLibrary.Conv_IntToString` playerNr)))
  (if local
    (set `self.LocalPlayerNr` playerNr)))

(event `self.changePlayerPos`
  (params (playerNr :type Integer) (x :type Integer) (y :type Integer))
  ;[1 1 1] Searching for actorNr in actors array
  (for _array_element (`self.Actors`)
    (`/Engine/EditorBlueprintResources/StandardMacros.CompareInt` (`/Game/Blueprints/Card.actorNr` _array_element) playerNr
      (:`==`
        (`/Game/Blueprints/Card.move` _array_element x y)))))

(event `self.changePlayerColor`
  (params (playerNr :type Integer) (col :type "Color Structure"))
  ;[1 1 1] Searching for actorNr in actors array
  (for _array_element (`self.Actors`)
    (`/Engine/EditorBlueprintResources/StandardMacros.CompareInt` (`/Game/Blueprints/Card.actorNr` _array_element) playerNr
      (:`==`
        (`/Game/Blueprints/Card.setColor` _array_element (`KismetMathLibrary.Conv_ColorToLinearColor` col) (== playerNr (`self.LocalPlayerNr`)))))))

(event `self.ReceiveTick`
  (params (DeltaSeconds :type "Float (single-precision)"))
  ;[1 1 1] We need to  change checker visibility only on UseGroups changes but doing that per frame for simplicity
  (`/Game/Blueprints/Board.updateCheckerVisibility` (`self.board`) (`self.useGroups`)))

(event `self.updateState`
  (params (state :type Integer) (stateStr :type String) (joinedRoomName :type String))
  ;[1 1 1] Set state string and copy of available rooms list
  (set `self.clientstateString` (`KismetStringLibrary.Concat_StrStr` (`KismetStringLibrary.Concat_StrStr` stateStr " ") joinedRoomName)))

(event `self.updateRoomList`
  (params (roomNames :type "Array of String (by ref)"))
  ;[1 1 1] Set state string and copy of available rooms list
  (set `self.rooms` roomNames))

(fn `UserConstructionScript`)