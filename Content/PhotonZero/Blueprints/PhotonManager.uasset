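; PhotonManager bridges Photon multiplayer to the game, tracking players, room names and client state.
; AddPlayer records each new player and spawns a NormalPlayer at StartPosition for remote ones, while ChangePlayerPos stores their transforms in index-matched arrays.
; BeginPlay sets a random user name and finds the TopDownCharacter, whose truncated integer transform Tick sends out.
; Tick's player loop is empty, so stored remote transforms are never applied here.
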(event `self.addPlayer`
  (params (playerNr :type Integer) (playerName :type String) (local :type Boolean))
  (bind _playerslocations (`self.PlayersLocations`))
  (bind _playersrotations (`self.PlayersRotations`))
  (bind _players (`self.Players`))
  (bind _playersnumber (`self.PlayersNumber`))
  ;[1 1 1] New Player Connected
  (if (not (`KismetArrayLibrary.Array_Contains` _playersnumber playerNr))
    (`KismetArrayLibrary.Array_Insert` _playersnumber playerNr)
    (if local
      (set `self.LocalPlayerNr` playerNr)
      (`KismetArrayLibrary.Array_Insert` _players null)
      (`KismetArrayLibrary.Array_Insert` _playerslocations (0.0 0.0 0.0))
      (`KismetArrayLibrary.Array_Insert` _playersrotations (struct))
      (set `self.ClientStateString` playerName)
      (else
        (bind _returnvalue (`|SpawnActorFromClass` "/Game/TopDown/Blueprints/NormalPlayer.NormalPlayer_C" (`self.GetTransform` (`self.StartPosition`)) true))
        (`KismetArrayLibrary.Array_Insert` _players _returnvalue)
        (`KismetArrayLibrary.Array_Insert` _playerslocations (`self.K2_GetActorLocation` _returnvalue))
        (`KismetArrayLibrary.Array_Insert` _playersrotations (`self.K2_GetActorRotation` _returnvalue))))))

(event `self.changePlayerPos`
  (params (playerNr :type Integer) (x :type Integer) (y :type Integer) (z :type Integer) (a :type Integer) (b :type Integer) (c :type Integer))
  ;[1 1 1] When Network Players Moved
  (if (not (== playerNr (`self.LocalPlayerNr`)))
    (for (_array_element _array_index) (`self.PlayersNumber`)
      (if (== playerNr _array_element)
        (`KismetArrayLibrary.Array_Set` (`self.PlayersLocations`) _array_index (`KismetMathLibrary.MakeVector` (`KismetMathLibrary.Conv_IntToDouble` x) (`KismetMathLibrary.Conv_IntToDouble` y) (`KismetMathLibrary.Conv_IntToDouble` z)))
        (`KismetArrayLibrary.Array_Set` (`self.PlayersRotations`) _array_index (`KismetMathLibrary.MakeRot` (`KismetMathLibrary.Conv_IntToDouble` a) (`KismetMathLibrary.Conv_IntToDouble` b) (`KismetMathLibrary.Conv_IntToDouble` c)))))))

(event `self.ReceiveBeginPlay`
  ;[1 1 1] Define the Player Character (Improve That)
  (`self.ChangeName` (`KismetStringLibrary.Concat_StrStr` "User" (`KismetStringLibrary.Conv_IntToString` (`KismetMathLibrary.RandomIntegerFromStream` 99999 (`KismetMathLibrary.MakeRandomStream` (`KismetMathLibrary.GetMillisecond` (`KismetMathLibrary.Now`)))))))
  (`KismetSystemLibrary.Delay` 1.0)
  (bind _outactors (`GameplayStatics.GetAllActorsOfClass` "/Game/TopDown/Blueprints/TopDownCharacter.TopDownCharacter_C"))
  (for _array_element _outactors
    (set `self.Character` _array_element)))

(event `self.updateState`
  (params (state :type Integer) (stateStr :type String) (joinedRoomName :type String))
  ;[1 1 1] Set state string and copy of available rooms list
  (set `self.ClientStateString` (`KismetStringLibrary.Concat_StrStr` stateStr joinedRoomName)))

(event `self.updateRoomList`
  (params (roomNames :type "Array of String (by ref)"))
  ;[1 1 1] Set state string and copy of available rooms list
  (set `self.rooms` roomNames))

(event `self.ReceiveTick`
  (params (DeltaSeconds :type "Float (single-precision)"))
  (bind _character (`self.Character`))
  ;[1 1 1] MoveChar
  (`/Engine/EditorBlueprintResources/StandardMacros.IsValid` _character
    (:`Is Valid`
      (`self.SetLocalPlayerPos` (`KismetMathLibrary.FTrunc` (.x (`self.K2_GetActorLocation` _character))) (`KismetMathLibrary.FTrunc` (.y (`self.K2_GetActorLocation` _character))) (`KismetMathLibrary.FTrunc` (.z (`self.K2_GetActorLocation` _character))) (`KismetMathLibrary.FTrunc` (.pitch (`self.K2_GetActorRotation` _character))) (`KismetMathLibrary.FTrunc` (.yaw (`self.K2_GetActorRotation` _character))) (`KismetMathLibrary.FTrunc` (.roll (`self.K2_GetActorRotation` _character))))
      (for _ (`self.Players`)
        _))))

(fn `MoveChar`
  (params (xPos :type Integer) (yPos :type Integer))
  (`self.SetLocalPlayerPos` xPos yPos))

(fn `UserConstructionScript`)